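; BP_HealthPot is a health potion item that heals the pawn using it by HealAmount.
; ItemEffect finds the instigator pawn's SAttributeComponent and, only when health is not full, calls ApplyHealthChange and returns its result.
; The EventGraph holds only disabled events and an unconnected older version of the heal logic with a debug health print, so none of it runs.
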(fn `ItemEffect`
  (params (InstigatorPawn :type "Pawn Object Reference"))
  (returns (ReturnValue :type Boolean))
  (bind _returnvalue (`self.GetComponentByClass` InstigatorPawn "/Script/ActionRogueL.SAttributeComponent"))
  (if (not (`SAttributeComponent.IsFullHealth` _returnvalue))
    (bind _returnvalue_2 (`SAttributeComponent.ApplyHealthChange` _returnvalue (`self.HealAmount`)))
    (return _returnvalue_2)))

(fn `UserConstructionScript`)