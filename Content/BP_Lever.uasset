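; BP_Lever is an interactable lever that relays interaction to a linked actor.
; Each Interact alternates, via FlipFlop, between playing and reversing a timeline that rotates the handle mesh between two angles.
; When the timeline finishes, it sends InteractMessage with the instigating pawn to DirectInteractActor if that actor implements SGameplayInterface.
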(event `SGameplayInterface.Interact`
  (params (InstigatorPawn :type "Pawn Object Reference"))
  (bind _isa (`/Engine/EditorBlueprintResources/StandardMacros.FlipFlop`)
    (:`A`
      (bind (_direction _alpha) (`Timeline|Timeline_Handle` :!label _label)
        (:`Update`
          (`SceneComponent.K2_SetRelativeRotation` (`self.HandleMesh`) (`KismetMathLibrary.RLerp` (struct :`Pitch` -30.0) (struct :`Pitch` 30.0) _alpha true) false false))
        (:`Finished`
          (if (`KismetSystemLibrary.DoesImplementInterface` (`self.DirectInteractActor`) "/Script/ActionRogueL.SGameplayInterface")
            (message `SGameplayInterface.Interact` (`self.DirectInteractActor`) InstigatorPawn)))))
    (:`B`
      (goto _label :!via `Reverse`))))

(fn `UserConstructionScript`)