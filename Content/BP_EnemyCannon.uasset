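; BP_EnemyCannon is an enemy turret that faces the player and fires magic projectiles.
; Every tick it snaps its whole actor rotation to look at the first player's pawn, with no smoothing or range check.
; When AutoActivate is set, BeginPlay starts a looping one-second timer that calls Shoot.
; Shoot spawns BP_MagicProjectile at the cannon's own transform, owned by the cannon and ignoring spawn collisions.
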(event `self.ReceiveBeginPlay`
  (if (`self.bAutoActivate`)
    (`KismetSystemLibrary.K2_SetTimerDelegate` (delegate `Shoot`) 1.0 true)))

(event `Shoot`
  (`|SpawnActorFromClass` "/Game/BP_MagicProjectile.BP_MagicProjectile_C" (`self.GetTransform`) "AlwaysSpawn" "OverrideRootScale" self null))

(event `self.ReceiveTick`
  (params (DeltaSeconds :type "Float (single-precision)"))
  (`self.K2_SetActorRotation` (`KismetMathLibrary.FindLookAtRotation` (`self.K2_GetActorLocation`) (`self.K2_GetActorLocation` (`GameplayStatics.GetPlayerPawn` 0)))))

(fn `UserConstructionScript`)